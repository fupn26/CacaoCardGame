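; Game state for a hot-seat card game that sets up the table and passes turns between CardGamePawn players.
; BeginPlay places Plantation and MarketX2 starter cards on the Board, deals three worker cards to each pawn's hand and fills the outer jungle slots from the JungleDeck.
; AdvanceTurnPlayer has the single player controller possess the next pawn, moves the shared board, deck and slots to its jump points, and re-enables worker card placement.
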(event EventBeginPlay
  (Utilities|FlowControl|Sequence
    (:then_0
      ;[1 1 1] kezdő jungel lapok spawnolása a board-ra
      (bind _returnvalue (Game|SpawnActorfromClass "/Game/CardGameTemplate/Blueprints/Cards/Plantation.Plantation_C" (Math|Conversions|ToTransform(Vector) (+ "0, 0, 0" 0)) "Undefined" 0 0))
      (Variables|/Game/CardGameTemplate/Blueprints/Cards/Card.Card_C|SetonBoard _returnvalue true)
      (Default|SetCardData _returnvalue (Utilities|Struct|MakeCardInfo "Card16" "" "/Game/CardGameTemplate/TexturesAndMaterials_Jungle/Plantation.Plantation" "/Engine/ArtTools/RenderToTexture/Textures/127grey.127grey" "/Game/CardGameTemplate/Blueprints/Cards/Plantation.Plantation_C"))
      (bind _outactors (Actor|GetAllActorsOfClass "/Game/CardGameTemplate/Blueprints/Board.Board_C"))
      (Default|Attachto _returnvalue (Variables|/Game/CardGameTemplate/Blueprints/BoardCardSlot.BoardCardSlot_C|GetScene (Utilities|Array|Get(acopy) (Variables|/Game/CardGameTemplate/Blueprints/Board.Board_C|GetSlots (Utilities|Array|Get(acopy) _outactors)) 54)) false)
      (Variables|/Game/CardGameTemplate/Blueprints/Cards/Card.Card_C|SetTargetTransform _returnvalue (Math|Transform|MakeTransform "0, 0, 0" "0, 0, 0" "1,1,1"))
      (Variables|/Game/CardGameTemplate/Blueprints/BoardCardSlot.BoardCardSlot_C|SetCard (Utilities|Array|Get(acopy) (Variables|/Game/CardGameTemplate/Blueprints/Board.Board_C|GetSlots (Utilities|Array|Get(acopy) _outactors)) 54) _returnvalue))
    (:then_1
      (bind _returnvalue_2 (Game|SpawnActorfromClass "/Game/CardGameTemplate/Blueprints/Cards/MarketX2.MarketX2_C" (Math|Conversions|ToTransform(Vector) (+ "0, 0, 0" 0)) "Undefined" 0 0))
      (Variables|/Game/CardGameTemplate/Blueprints/Cards/Card.Card_C|SetonBoard _returnvalue_2 true)
      (Default|SetCardData _returnvalue_2 (Utilities|Struct|MakeCardInfo "Card16" "" "/Game/CardGameTemplate/TexturesAndMaterials_Jungle/MarketX2.MarketX2" "/Engine/ArtTools/RenderToTexture/Textures/127grey.127grey" "/Game/CardGameTemplate/Blueprints/Cards/MarketX2.MarketX2_C"))
      (Default|Attachto _returnvalue_2 (Variables|/Game/CardGameTemplate/Blueprints/BoardCardSlot.BoardCardSlot_C|GetScene (Utilities|Array|Get(acopy) (Variables|/Game/CardGameTemplate/Blueprints/Board.Board_C|GetSlots (Utilities|Array|Get(acopy) _outactors)) 45)) false)
      (Variables|/Game/CardGameTemplate/Blueprints/Cards/Card.Card_C|SetTargetTransform _returnvalue_2 (Math|Transform|MakeTransform "0, 0, 0" "0, 0, 0" "1,1,1"))
      (Variables|/Game/CardGameTemplate/Blueprints/BoardCardSlot.BoardCardSlot_C|SetCard (Utilities|Array|Get(acopy) (Variables|/Game/CardGameTemplate/Blueprints/Board.Board_C|GetSlots (Utilities|Array|Get(acopy) _outactors)) 45) _returnvalue_2))
    (:then_2
      (bind _outactors_2 (Actor|GetAllActorsOfClass "/Game/CardGameTemplate/Blueprints/CardGamePawn.CardGamePawn_C"))
      (bind _output_get (Variables|Default|SetPlayerPawns _outactors_2))
      (Pawn|Possess (Game|GetPlayerController 0) (Utilities|Array|Get(acopy) _output_get))
      (Utilities|FlowControl|Sequence
        (:then_0
          ;[1 1 1] Jungle deck object referencia ráállítása a világban található jungle deck-re majd a kezdeni poziciójának megadása
          (bind _outactors_3 (Actor|GetAllActorsOfClass "/Game/CardGameTemplate/Blueprints/JungleDeck.JungleDeck_C"))
          (bind _output_get_2 (Variables|Default|SetJungleDeck (Utilities|Array|Get(acopy) _outactors_3)))
          (Transformation|SetActorLocationAndRotation _output_get_2 (Transformation|GetWorldLocation (Variables|/Game/CardGameTemplate/Blueprints/CardGamePawn.CardGamePawn_C|GetJungleDeckJumpPoint (Utilities|Array|Get(acopy) _output_get))) (Transformation|GetWorldRotation (Variables|/Game/CardGameTemplate/Blueprints/CardGamePawn.CardGamePawn_C|GetJungleDeckJumpPoint (Utilities|Array|Get(acopy) _output_get)))))
        (:then_1
          ;[1 1 1] Board object referencia ráállítása a világban található Board-ra majd a kezdeni poziciójának megadása
          (bind _outactors_4 (Actor|GetAllActorsOfClass "/Game/CardGameTemplate/Blueprints/Board.Board_C"))
          (bind _output_get_3 (Variables|Default|SetBoard (Utilities|Array|Get(acopy) _outactors_4)))
          (Transformation|SetActorLocationAndRotation _output_get_3 (Transformation|GetWorldLocation (Variables|/Game/CardGameTemplate/Blueprints/CardGamePawn.CardGamePawn_C|GetBoardJumppoint (Utilities|Array|Get(acopy) _output_get))) (Transformation|GetWorldRotation (Variables|/Game/CardGameTemplate/Blueprints/CardGamePawn.CardGamePawn_C|GetBoardJumppoint (Utilities|Array|Get(acopy) _output_get)))))
        (:then_2
          ;[1 1 1] első körben huzható 3 lap hozzáadása a kézhez
          (bind _outactors_5 (Actor|GetAllActorsOfClass "/Game/CardGameTemplate/Blueprints/WorkerDeck.WorkerDeck_C"))
          (for (_array_element _array_index) _output_get
            (for _index (range 0 2)
              (if (Utilities|IsValid (Variables|/Game/CardGameTemplate/Blueprints/CardGamePawn.CardGamePawn_C|GetHand _array_element))
                (Variables|/Game/CardGameTemplate/Blueprints/Hand.Hand_C|SetcanDrawWorkerCard (Variables|/Game/CardGameTemplate/Blueprints/CardGamePawn.CardGamePawn_C|GetHand _array_element) true)
                (Default|DrawfromDeck (Variables|/Game/CardGameTemplate/Blueprints/CardGamePawn.CardGamePawn_C|GetHand _array_element) (Utilities|Array|Get(acopy) _outactors_5 _array_index) false)
                (Variables|/Game/CardGameTemplate/Blueprints/Hand.Hand_C|SetcanDrawWorkerCard (Variables|/Game/CardGameTemplate/Blueprints/CardGamePawn.CardGamePawn_C|GetHand _array_element) false)))))
        (:then_4
          ;[1 1 1] JungleCardslot objektum refenciák beállítása és kezdeti pozíciójuknak beállítása
          (bind _outactors_6 (Actor|GetAllActorsOfClass "/Game/CardGameTemplate/Blueprints/OuterJungleSlot.OuterJungleSlot_C"))
          (Utilities|FlowControl|Sequence
            (:then_0
              (bind _output_get_4 (Variables|Default|SetOuterJungleCardSlot1 (Utilities|Array|Get(acopy) _outactors_6)))
              (Transformation|SetActorLocationAndRotation _output_get_4 (Transformation|GetWorldLocation (Variables|/Game/CardGameTemplate/Blueprints/CardGamePawn.CardGamePawn_C|GetOuterJungleslotJumpPoint (Utilities|Array|Get(acopy) _output_get))) (Transformation|GetWorldRotation (Variables|/Game/CardGameTemplate/Blueprints/CardGamePawn.CardGamePawn_C|GetOuterJungleslotJumpPoint (Utilities|Array|Get(acopy) _output_get)))))
            (:then_1
              (bind _output_get_5 (Variables|Default|SetOuterJungleCardSlot2 (Utilities|Array|Get(acopy) _outactors_6 1)))
              (Transformation|SetActorLocationAndRotation _output_get_5 (Transformation|GetWorldLocation (Variables|/Game/CardGameTemplate/Blueprints/CardGamePawn.CardGamePawn_C|GetOuterJungleslotJumpPoint1 (Utilities|Array|Get(acopy) _output_get))) (Transformation|GetWorldRotation (Variables|/Game/CardGameTemplate/Blueprints/CardGamePawn.CardGamePawn_C|GetOuterJungleslotJumpPoint1 (Utilities|Array|Get(acopy) _output_get)))))))))
    (:then_4
      ;[1 1 1] kezdő kitett jungel lapok hozzáadása az outer jungle card slotokhoz
      (bind _outactors_7 (Actor|GetAllActorsOfClass "/Game/CardGameTemplate/Blueprints/OuterJungleSlot.OuterJungleSlot_C"))
      (for _array_element_2 _outactors_7
        (bind _outactors_8 (Actor|GetAllActorsOfClass "/Game/CardGameTemplate/Blueprints/JungleDeck.JungleDeck_C"))
        (bind _topcard (Default|PopLastCard (Utilities|Array|Get(acopy) _outactors_8)))
        (Default|Attachto _topcard (Variables|/Game/CardGameTemplate/Blueprints/BoardCardSlot.BoardCardSlot_C|GetScene _array_element_2) false)
        (Variables|/Game/CardGameTemplate/Blueprints/Cards/Card.Card_C|SetTargetTransform _topcard (Math|Transform|MakeTransform "0, 0, 0" "0, 0, 0" "1,1,1"))
        (Variables|/Game/CardGameTemplate/Blueprints/BoardCardSlot.BoardCardSlot_C|SetCard _array_element_2 _topcard)))))

(fn ConstructionScript)

(fn AdvanceTurnPlayer
  ;[1 1 1] Kör léptetése: megfelelő playerpawn írányitásának léptetése
  (Variables|Default|SetTurnPlayer (select (== (+ (Variables|Default|GetTurnPlayer) 1) (Variables|Default|GetNumPlayers)) 0 (+ (Variables|Default|GetTurnPlayer) 1)))
  (Pawn|UnPossess (Game|GetPlayerController 0))
  (Pawn|Possess (Game|GetPlayerController 0) (Utilities|Array|Get(acopy) (Variables|Default|GetPlayerPawns) (Variables|Default|GetTurnPlayer)))
  (Utilities|FlowControl|Sequence
    (:then_0
      ;[1 1 1] Jungel pakli ugratása a megfelelő játékoshoz
      (Transformation|SetActorLocationAndRotation (Variables|Default|GetJungleDeck) (Transformation|GetWorldLocation (Variables|/Game/CardGameTemplate/Blueprints/CardGamePawn.CardGamePawn_C|GetJungleDeckJumpPoint (Utilities|Array|Get(acopy) (Variables|Default|GetPlayerPawns) (Variables|Default|GetTurnPlayer)))) (Transformation|GetWorldRotation (Variables|/Game/CardGameTemplate/Blueprints/CardGamePawn.CardGamePawn_C|GetJungleDeckJumpPoint (Utilities|Array|Get(acopy) (Variables|Default|GetPlayerPawns) (Variables|Default|GetTurnPlayer))))))
    (:then_1
      ;[1 1 1] Board ugratása a megfelelő játékoshoz
      (Transformation|SetActorLocationAndRotation (Variables|Default|GetBoard) (Transformation|GetWorldLocation (Variables|/Game/CardGameTemplate/Blueprints/CardGamePawn.CardGamePawn_C|GetBoardJumppoint (Utilities|Array|Get(acopy) (Variables|Default|GetPlayerPawns) (Variables|Default|GetTurnPlayer)))) (Transformation|GetWorldRotation (Variables|/Game/CardGameTemplate/Blueprints/CardGamePawn.CardGamePawn_C|GetBoardJumppoint (Utilities|Array|Get(acopy) (Variables|Default|GetPlayerPawns) (Variables|Default|GetTurnPlayer))))))
    (:then_2
      ;[1 1 1] körváltáskor beállítjuk hogy az adott player ismét tudjon lerakni munkáslapot
      (Variables|/Game/CardGameTemplate/Blueprints/Hand.Hand_C|SetcanPlaceWorkerCard (Variables|/Game/CardGameTemplate/Blueprints/CardGamePawn.CardGamePawn_C|GetHand (Utilities|Array|Get(acopy) (Variables|Default|GetPlayerPawns) (Variables|Default|GetTurnPlayer))) true))
    (:then_4
      ;[1 1 1] outer jungle helyek ugratása körönként a mgefelelő játékoshoz
      (Utilities|FlowControl|Sequence
        (:then_0
          (Transformation|SetActorLocationAndRotation (Variables|Default|GetOuterJungleCardSlot1) (Transformation|GetWorldLocation (Variables|/Game/CardGameTemplate/Blueprints/CardGamePawn.CardGamePawn_C|GetOuterJungleslotJumpPoint (Utilities|Array|Get(acopy) (Variables|Default|GetPlayerPawns) (Variables|Default|GetTurnPlayer)))) (Transformation|GetWorldRotation (Variables|/Game/CardGameTemplate/Blueprints/CardGamePawn.CardGamePawn_C|GetOuterJungleslotJumpPoint (Utilities|Array|Get(acopy) (Variables|Default|GetPlayerPawns) (Variables|Default|GetTurnPlayer))))))
        (:then_1
          (Transformation|SetActorLocationAndRotation (Variables|Default|GetOuterJungleCardSlot2) (Transformation|GetWorldLocation (Variables|/Game/CardGameTemplate/Blueprints/CardGamePawn.CardGamePawn_C|GetOuterJungleslotJumpPoint1 (Utilities|Array|Get(acopy) (Variables|Default|GetPlayerPawns) (Variables|Default|GetTurnPlayer)))) (Transformation|GetWorldRotation (Variables|/Game/CardGameTemplate/Blueprints/CardGamePawn.CardGamePawn_C|GetOuterJungleslotJumpPoint1 (Utilities|Array|Get(acopy) (Variables|Default|GetPlayerPawns) (Variables|Default|GetTurnPlayer))))))))))