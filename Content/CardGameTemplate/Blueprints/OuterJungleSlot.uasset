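; OuterJungleSlot is a card game slot actor that lets the player select the card it holds by clicking its highlight mesh.
; A click with a valid card stores the card and slot on the player pawn's Hand, which handles placement from there per the author's comment.
; It then hides the highlight on all OuterJungleSlot actors and shows its own, leaving one slot highlighted.
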(event OnClicked(HighlightMesh)
  (params (TouchedComponent :type Primitive%20Component%20Object%20Reference) (ButtonPressed :type Key%20Structure :default "None"))
  ;[1 1 1] Ha rákattintunk a kitett slotra akkor beállítjuk a hand clicket card változóját az adott kártyára,és innentől a hand kezeli a kártyalerakást,valamint iss is kezeljük a highlight mesh láthatóságát
  (bind _ascard_game_pawn (Utilities|Casting|CastToCardGamePawn (Game|Player|GetPlayerPawn 0)))
  (Variables|Default|SetPlayerPawn _ascard_game_pawn)
  (Utilities|IsValid (Variables|Default|GetCard)
    (:Is%20Valid
      (Utilities|IsValid (Variables|/Game/CardGameTemplate/Blueprints/Hand.Hand_C|GetClickedCard (Variables|/Game/CardGameTemplate/Blueprints/CardGamePawn.CardGamePawn_C|GetHand (Variables|Default|GetPlayerPawn)))
        (:Is%20Valid
          (Variables|/Game/CardGameTemplate/Blueprints/Hand.Hand_C|SetClickedCard (Variables|/Game/CardGameTemplate/Blueprints/CardGamePawn.CardGamePawn_C|GetHand (Variables|Default|GetPlayerPawn)) 0))
        (:Is%20Not%20Valid
          _))
      (Variables|/Game/CardGameTemplate/Blueprints/Hand.Hand_C|SetClickedCard (Variables|/Game/CardGameTemplate/Blueprints/CardGamePawn.CardGamePawn_C|GetHand (Variables|Default|GetPlayerPawn)) (Variables|Default|GetCard))
      (Variables|/Game/CardGameTemplate/Blueprints/Hand.Hand_C|SetClickedCardOuterSlot (Variables|/Game/CardGameTemplate/Blueprints/CardGamePawn.CardGamePawn_C|GetHand (Variables|Default|GetPlayerPawn)) self)
      (Utilities|Casting|CastToCardGameGameState (Game|GetGameState))
      (bind _outactors (Actor|GetAllActorsOfClass "OuterJungleSlot_C"))
      (for _array_element _outactors
        (Rendering|SetVisibility (Variables|/Game/CardGameTemplate/Blueprints/BoardCardSlot.BoardCardSlot_C|GetHighlightMesh _array_element) false false))
      (Rendering|SetVisibility (Variables|Default|GetHighlightMesh) true true))))

(event EventBeginPlay)

(event Collision|EventActorBeginOverlap
  (params (OtherActor :type Actor%20Object%20Reference)))

(event EventTick
  (params (DeltaSeconds :type Float%20%28single-precision%29)))

(fn ConstructionScript
  (|CallParentFunction))