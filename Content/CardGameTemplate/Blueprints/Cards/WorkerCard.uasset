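; Worker card actor whose four clickable sides each activate an adjacent jungle card.
; A click only acts when the card's text, Blue or Red, matches the game state's TurnPlayer.
; It stretches the side's child collision boxes to overlap the neighbouring JungleCard and trigger its effect, shrinking them back if none is hit so the side stays reusable.
; Hovering a side toggles that component's visibility as a highlight.
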(event OnBeginCursorOver(Bottom)
  (params (TouchedComponent :type Primitive%20Component%20Object%20Reference))
  (Rendering|SetVisibility TouchedComponent true false))

(event OnEndCursorOver(Bottom)
  (params (TouchedComponent :type Primitive%20Component%20Object%20Reference))
  (Rendering|SetVisibility TouchedComponent false false))

(event OnBeginCursorOver(Left)
  (params (TouchedComponent :type Primitive%20Component%20Object%20Reference))
  (Rendering|SetVisibility TouchedComponent true false))

(event OnEndCursorOver(Left)
  (params (TouchedComponent :type Primitive%20Component%20Object%20Reference))
  (Rendering|SetVisibility TouchedComponent false false))

(event OnBeginCursorOver(Right)
  (params (TouchedComponent :type Primitive%20Component%20Object%20Reference))
  (Rendering|SetVisibility TouchedComponent true false))

(event OnEndCursorOver(Right)
  (params (TouchedComponent :type Primitive%20Component%20Object%20Reference))
  (Rendering|SetVisibility TouchedComponent false false))

(event OnClicked(Top)
  (params (TouchedComponent :type Primitive%20Component%20Object%20Reference) (ButtonPressed :type Key%20Structure :default "None"))
  (bind _cardtext (Variables|Default|GetCardText))
  (bind _text (Variables|/Script/Engine.TextRenderComponent|GetText _cardtext))
  (bind _returnvalue (Utilities|String|ToString(Text) _text))
  ;[1 1 1] onclicked akciók kezelése a kártyalap oldalain, kék kártyát kék pirosat csak a piros játékos tud aktiválni, katintás hatására megnöveljük az adott oldalhoz adott collision boxot ami így hozzá fog érni a szomszédos jungel laphoz és aktiválja a jungel lap effektjét
  (if (Utilities|Enum|Equal(Enum) _returnvalue (Utilities|String|MakeLiteralString "Blue"))
    (bind _ascard_game_game_state (Utilities|Casting|CastToCardGameGameState (Game|GetGameState)))
    (if (== (Variables|/Game/CardGameTemplate/Blueprints/CardGameGameState.CardGameGameState_C|GetTurnPlayer _ascard_game_game_state) 0)
      (for _array_element (Components|GetChildrenComponents (Variables|Default|GetTop) false) :!label _label
        (bind _asbox_collision (Utilities|Casting|CastToBoxComponent _array_element))
        (Variables|/Script/Engine.PrimitiveComponent|SetbGenerateOverlapEvents _asbox_collision true)
        (Transformation|SetRelativeScale3D _asbox_collision "1.000000,20.000000,1.000000")
        ;[1 1 1] Ha a collision box növekedése közben nem talált el jungel lapot akkor visszaálítjuk ez eredeti méretére, hogy ha késöbb lap kerülne mellé akkor újra aktiválni tudjuk és ne automatikusan aktiválódjon ha jungel lapot teszünk mellé
        (if (not (Utilities|Array|IsValidIndex (Collision|GetOverlappingActors _asbox_collision "/Game/CardGameTemplate/Blueprints/Cards/JungleCard.JungleCard_C" :!class /Script/Engine.PrimitiveComponent)))
          (Transformation|SetRelativeScale3D _asbox_collision "1.000000,1.000000,1.000000"))))
    (elif (Utilities|Enum|Equal(Enum) _returnvalue (Utilities|String|MakeLiteralString "Red"))
      (bind _ascard_game_game_state_2 (Utilities|Casting|CastToCardGameGameState (Game|GetGameState)))
      (if (== (Variables|/Game/CardGameTemplate/Blueprints/CardGameGameState.CardGameGameState_C|GetTurnPlayer _ascard_game_game_state_2) 1)
        (goto _label)))))

(event OnClicked(Bottom)
  (params (TouchedComponent :type Primitive%20Component%20Object%20Reference) (ButtonPressed :type Key%20Structure :default "None"))
  (bind _cardtext (Variables|Default|GetCardText))
  (bind _text (Variables|/Script/Engine.TextRenderComponent|GetText _cardtext))
  (bind _returnvalue (Utilities|String|ToString(Text) _text))
  ;[1 1 1] onclicked akciók kezelése a kártyalap oldalain, kék kártyát kék pirosat csak a piros játékos tud aktiválni, katintás hatására megnöveljük az adott oldalhoz adott collision boxot ami így hozzá fog érni a szomszédos jungel laphoz és aktiválja a jungel lap effektjét
  (if (Utilities|Enum|Equal(Enum) _returnvalue (Utilities|String|MakeLiteralString "Blue"))
    (bind _ascard_game_game_state (Utilities|Casting|CastToCardGameGameState (Game|GetGameState)))
    (if (== (Variables|/Game/CardGameTemplate/Blueprints/CardGameGameState.CardGameGameState_C|GetTurnPlayer _ascard_game_game_state) 0)
      (for _array_element (Components|GetChildrenComponents (Variables|Default|GetBottom) false) :!label _label
        (bind _asbox_collision (Utilities|Casting|CastToBoxComponent _array_element))
        (Variables|/Script/Engine.PrimitiveComponent|SetbGenerateOverlapEvents _asbox_collision true)
        (Transformation|SetRelativeScale3D _asbox_collision "1.000000,20.000000,1.000000")
        ;[1 1 1] Ha a collision box növekedése közben nem talált el jungel lapot akkor visszaálítjuk ez eredeti méretére, hogy ha késöbb lap kerülne mellé akkor újra aktiválni tudjuk és ne automatikusan aktiválódjon ha jungel lapot teszünk mellé
        (if (not (Utilities|Array|IsValidIndex (Collision|GetOverlappingActors _asbox_collision "/Game/CardGameTemplate/Blueprints/Cards/JungleCard.JungleCard_C" :!class /Script/Engine.PrimitiveComponent)))
          (Transformation|SetRelativeScale3D _asbox_collision "1.000000,1.000000,1.000000"))))
    (elif (Utilities|Enum|Equal(Enum) _returnvalue (Utilities|String|MakeLiteralString "Red"))
      (bind _ascard_game_game_state_2 (Utilities|Casting|CastToCardGameGameState (Game|GetGameState)))
      (if (== (Variables|/Game/CardGameTemplate/Blueprints/CardGameGameState.CardGameGameState_C|GetTurnPlayer _ascard_game_game_state_2) 1)
        (goto _label)))))

(event OnClicked(Left)
  (params (TouchedComponent :type Primitive%20Component%20Object%20Reference) (ButtonPressed :type Key%20Structure :default "None"))
  (bind _cardtext (Variables|Default|GetCardText))
  (bind _text (Variables|/Script/Engine.TextRenderComponent|GetText _cardtext))
  (bind _returnvalue (Utilities|String|ToString(Text) _text))
  ;[1 1 1] onclicked akciók kezelése a kártyalap oldalain, kék kártyát kék pirosat csak a piros játékos tud aktiválni, katintás hatására megnöveljük az adott oldalhoz adott collision boxot ami így hozzá fog érni a szomszédos jungel laphoz és aktiválja a jungel lap effektjét
  (if (Utilities|Enum|Equal(Enum) _returnvalue (Utilities|String|MakeLiteralString "Blue"))
    (bind _ascard_game_game_state (Utilities|Casting|CastToCardGameGameState (Game|GetGameState)))
    (if (== (Variables|/Game/CardGameTemplate/Blueprints/CardGameGameState.CardGameGameState_C|GetTurnPlayer _ascard_game_game_state) 0)
      (for _array_element (Components|GetChildrenComponents (Variables|Default|GetLeft) false) :!label _label
        (bind _asbox_collision (Utilities|Casting|CastToBoxComponent _array_element))
        (Variables|/Script/Engine.PrimitiveComponent|SetbGenerateOverlapEvents _asbox_collision true)
        (Transformation|SetRelativeScale3D _asbox_collision "1.000000,20.000000,1.000000")
        ;[1 1 1] Ha a collision box növekedése közben nem talált el jungel lapot akkor visszaálítjuk ez eredeti méretére, hogy ha késöbb lap kerülne mellé akkor újra aktiválni tudjuk és ne automatikusan aktiválódjon ha jungel lapot teszünk mellé
        (if (not (Utilities|Array|IsValidIndex (Collision|GetOverlappingActors _asbox_collision "/Game/CardGameTemplate/Blueprints/Cards/JungleCard.JungleCard_C" :!class /Script/Engine.PrimitiveComponent)))
          (Transformation|SetRelativeScale3D _asbox_collision "1.000000,1.000000,1.000000"))))
    (elif (Utilities|Enum|Equal(Enum) _returnvalue (Utilities|String|MakeLiteralString "Red"))
      (bind _ascard_game_game_state_2 (Utilities|Casting|CastToCardGameGameState (Game|GetGameState)))
      (if (== (Variables|/Game/CardGameTemplate/Blueprints/CardGameGameState.CardGameGameState_C|GetTurnPlayer _ascard_game_game_state_2) 1)
        (goto _label)))))

(event OnClicked(Right)
  (params (TouchedComponent :type Primitive%20Component%20Object%20Reference) (ButtonPressed :type Key%20Structure :default "None"))
  (bind _cardtext (Variables|Default|GetCardText))
  (bind _text (Variables|/Script/Engine.TextRenderComponent|GetText _cardtext))
  (bind _returnvalue (Utilities|String|ToString(Text) _text))
  ;[1 1 1] onclicked akciók kezelése a kártyalap oldalain, kék kártyát kék pirosat csak a piros játékos tud aktiválni, katintás hatására megnöveljük az adott oldalhoz adott collision boxot ami így hozzá fog érni a szomszédos jungel laphoz és aktiválja a jungel lap effektjét
  (if (Utilities|Enum|Equal(Enum) _returnvalue (Utilities|String|MakeLiteralString "Blue"))
    (bind _ascard_game_game_state (Utilities|Casting|CastToCardGameGameState (Game|GetGameState)))
    (if (== (Variables|/Game/CardGameTemplate/Blueprints/CardGameGameState.CardGameGameState_C|GetTurnPlayer _ascard_game_game_state) 0)
      (for _array_element (Components|GetChildrenComponents (Variables|Default|GetRight) false) :!label _label
        (bind _asbox_collision (Utilities|Casting|CastToBoxComponent _array_element))
        (Variables|/Script/Engine.PrimitiveComponent|SetbGenerateOverlapEvents _asbox_collision true)
        (Transformation|SetRelativeScale3D _asbox_collision "1.000000,20.000000,1.000000")
        ;[1 1 1] Ha a collision box növekedése közben nem talált el jungel lapot akkor visszaálítjuk ez eredeti méretére, hogy ha késöbb lap kerülne mellé akkor újra aktiválni tudjuk és ne automatikusan aktiválódjon ha jungel lapot teszünk mellé
        (if (not (Utilities|Array|IsValidIndex (Collision|GetOverlappingActors _asbox_collision "/Game/CardGameTemplate/Blueprints/Cards/JungleCard.JungleCard_C" :!class /Script/Engine.PrimitiveComponent)))
          (Transformation|SetRelativeScale3D _asbox_collision "1.000000,1.000000,1.000000"))))
    (elif (Utilities|Enum|Equal(Enum) _returnvalue (Utilities|String|MakeLiteralString "Red"))
      (bind _ascard_game_game_state_2 (Utilities|Casting|CastToCardGameGameState (Game|GetGameState)))
      (if (== (Variables|/Game/CardGameTemplate/Blueprints/CardGameGameState.CardGameGameState_C|GetTurnPlayer _ascard_game_game_state_2) 1)
        (goto _label)))))

(event OnBeginCursorOver(Top)
  (params (TouchedComponent :type Primitive%20Component%20Object%20Reference))
  (Rendering|SetVisibility TouchedComponent true false))

(event OnEndCursorOver(Top)
  (params (TouchedComponent :type Primitive%20Component%20Object%20Reference))
  (Rendering|SetVisibility TouchedComponent false false))

(event EventBeginPlay
  (|CallParentFunction) ; This node is disabled and will not be called.\nDrag off pins to build functionality.
)

(event Collision|EventActorBeginOverlap
  (params (OtherActor :type Actor%20Object%20Reference)))

(event EventTick
  (params (DeltaSeconds :type Float%20%28single-precision%29))
  (|CallParentFunction DeltaSeconds) ; This node is disabled and will not be called.\nDrag off pins to build functionality.
)

(fn ConstructionScript
  (|CallParentFunction))