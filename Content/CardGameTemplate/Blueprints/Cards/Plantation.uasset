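; Plantation is a card Blueprint in the card game template whose effect grants cacao to a player.
; ActivateEffect looks up the pawn for the given player index in the CardGameGameState and adds the card's Cacao value to that pawn's total, capped at a hard-coded maximum of five.
; It then calls OnCacaoChanged on the pawn to signal the new total.
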(event EventBeginPlay
  (|CallParentFunction) ; This node is disabled and will not be called.\nDrag off pins to build functionality.
)

(event Collision|EventActorBeginOverlap
  (params (OtherActor :type Actor%20Object%20Reference))
  (|CallParentFunction OtherActor) ; This node is disabled and will not be called.\nDrag off pins to build functionality.
)

(event EventTick
  (params (DeltaSeconds :type Float%20%28single-precision%29))
  (|CallParentFunction DeltaSeconds) ; This node is disabled and will not be called.\nDrag off pins to build functionality.
)

(event EventActivateEffect
  (params (PlayerIndex :type Integer))
  (bind _ascard_game_game_state (Utilities|Casting|CastToCardGameGameState (Game|GetGameState)))
  (if (> (+ (Variables|/Game/CardGameTemplate/Blueprints/CardGamePawn.CardGamePawn_C|GetCacao (Utilities|Array|Get(acopy) (Variables|/Game/CardGameTemplate/Blueprints/CardGameGameState.CardGameGameState_C|GetPlayerPawns _ascard_game_game_state) PlayerIndex)) (Variables|Default|GetCacao)) 5)
    (Variables|/Game/CardGameTemplate/Blueprints/CardGamePawn.CardGamePawn_C|SetCacao (Utilities|Array|Get(acopy) (Variables|/Game/CardGameTemplate/Blueprints/CardGameGameState.CardGameGameState_C|GetPlayerPawns _ascard_game_game_state) PlayerIndex) 5)
    (else
      (Variables|/Game/CardGameTemplate/Blueprints/CardGamePawn.CardGamePawn_C|SetCacao (Utilities|Array|Get(acopy) (Variables|/Game/CardGameTemplate/Blueprints/CardGameGameState.CardGameGameState_C|GetPlayerPawns _ascard_game_game_state) PlayerIndex) (+ (Variables|/Game/CardGameTemplate/Blueprints/CardGamePawn.CardGamePawn_C|GetCacao (Utilities|Array|Get(acopy) (Variables|/Game/CardGameTemplate/Blueprints/CardGameGameState.CardGameGameState_C|GetPlayerPawns _ascard_game_game_state) PlayerIndex)) (Variables|Default|GetCacao)))))
  (Default|OnCacaoChanged (Utilities|Array|Get(acopy) (Variables|/Game/CardGameTemplate/Blueprints/CardGameGameState.CardGameGameState_C|GetPlayerPawns _ascard_game_game_state) PlayerIndex)))

(fn ConstructionScript
  (|CallParentFunction))