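; SunJungle is a card Blueprint in the card game template whose effect grants its player one sun.
; ActivateEffect looks up the player's pawn in CardGameGameState by player index and increments its Suns only while the result stays at three or fewer.
; On a successful gain it prints the new count and calls the pawn's OnSunChanged.
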(event EventBeginPlay
  (|CallParentFunction) ; This node is disabled and will not be called.\nDrag off pins to build functionality.
)

(event Collision|EventActorBeginOverlap
  (params (OtherActor :type Actor%20Object%20Reference))
  (|CallParentFunction OtherActor) ; This node is disabled and will not be called.\nDrag off pins to build functionality.
)

(event EventTick
  (params (DeltaSeconds :type Float%20%28single-precision%29))
  (|CallParentFunction DeltaSeconds) ; This node is disabled and will not be called.\nDrag off pins to build functionality.
)

(event EventActivateEffect
  (params (PlayerIndex :type Integer))
  (bind _ascard_game_game_state (Utilities|Casting|CastToCardGameGameState (Game|GetGameState)))
  (if (not (> (+ (Variables|/Game/CardGameTemplate/Blueprints/CardGamePawn.CardGamePawn_C|GetSuns (Utilities|Array|Get(acopy) (Variables|/Game/CardGameTemplate/Blueprints/CardGameGameState.CardGameGameState_C|GetPlayerPawns _ascard_game_game_state) PlayerIndex)) 1) 3))
    (bind _output_get (Variables|/Game/CardGameTemplate/Blueprints/CardGamePawn.CardGamePawn_C|SetSuns (Utilities|Array|Get(acopy) (Variables|/Game/CardGameTemplate/Blueprints/CardGameGameState.CardGameGameState_C|GetPlayerPawns _ascard_game_game_state) PlayerIndex) (+ (Variables|/Game/CardGameTemplate/Blueprints/CardGamePawn.CardGamePawn_C|GetSuns (Utilities|Array|Get(acopy) (Variables|/Game/CardGameTemplate/Blueprints/CardGameGameState.CardGameGameState_C|GetPlayerPawns _ascard_game_game_state) PlayerIndex)) 1)))
    (Development|PrintString (Utilities|String|ToString(Integer) _output_get))
    (Default|OnSunChanged (Utilities|Array|Get(acopy) (Variables|/Game/CardGameTemplate/Blueprints/CardGameGameState.CardGameGameState_C|GetPlayerPawns _ascard_game_game_state) PlayerIndex))))

(fn ConstructionScript
  (|CallParentFunction))