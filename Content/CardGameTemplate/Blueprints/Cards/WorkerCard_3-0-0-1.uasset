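; Worker card Blueprint (3-0-0-1 variant) that activates neighboring jungle cards for the player who owns the worker.
; Four box components each run the same overlap check, requiring both this card and the overlapped JungleCard to be on the board.
; Ownership comes from comparing the CardText string: "Blue" calls ActivateEffect with 0, "Red" with 1.
; The overlap logic is duplicated per box rather than shared in a function.
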(event OnComponentBeginOverlap(Box)
  (params (OverlappedComponent :type Primitive%20Component%20Object%20Reference) (OtherActor :type Actor%20Object%20Reference) (OtherComp :type Primitive%20Component%20Object%20Reference) (OtherBodyIndex :type Integer) (bFromSweep :type Boolean) (SweepResult :type Hit%20Result%20Structure%20%28by%20ref%29))
  (bind _cardtext (Variables|Default|GetCardText))
  (bind _text (Variables|/Script/Engine.TextRenderComponent|GetText _cardtext))
  (bind _returnvalue (Utilities|String|ToString(Text) _text))
  ;[1 1 1] az érintet jungel kártya aktiválása és az effect-jének alkalmazása arra a játékosra amelyiknek tartozik az adott munkás lap
  (if (Variables|Default|GetonBoard)
    (bind _asjungle_card (Utilities|Casting|CastToJungleCard OtherActor))
    (if (Variables|/Game/CardGameTemplate/Blueprints/Cards/Card.Card_C|GetonBoard _asjungle_card)
      (if (Utilities|Enum|Equal(Enum) _returnvalue (Utilities|String|MakeLiteralString "Blue"))
        (Default|ActivateEffect _asjungle_card)
        (elif (Utilities|Enum|Equal(Enum) _returnvalue (Utilities|String|MakeLiteralString "Red"))
          (Default|ActivateEffect _asjungle_card 1))))))

(event OnComponentBeginOverlap(Box1)
  (params (OverlappedComponent :type Primitive%20Component%20Object%20Reference) (OtherActor :type Actor%20Object%20Reference) (OtherComp :type Primitive%20Component%20Object%20Reference) (OtherBodyIndex :type Integer) (bFromSweep :type Boolean) (SweepResult :type Hit%20Result%20Structure%20%28by%20ref%29))
  (bind _cardtext (Variables|Default|GetCardText))
  (bind _text (Variables|/Script/Engine.TextRenderComponent|GetText _cardtext))
  (bind _returnvalue (Utilities|String|ToString(Text) _text))
  ;[1 1 1] az érintet jungel kártya aktiválása és az effect-jének alkalmazása arra a játékosra amelyiknek tartozik az adott munkás lap
  (if (Variables|Default|GetonBoard)
    (bind _asjungle_card (Utilities|Casting|CastToJungleCard OtherActor))
    (if (Variables|/Game/CardGameTemplate/Blueprints/Cards/Card.Card_C|GetonBoard _asjungle_card)
      (if (Utilities|Enum|Equal(Enum) _returnvalue (Utilities|String|MakeLiteralString "Blue"))
        (Default|ActivateEffect _asjungle_card)
        (elif (Utilities|Enum|Equal(Enum) _returnvalue (Utilities|String|MakeLiteralString "Red"))
          (Default|ActivateEffect _asjungle_card 1))))))

(event OnComponentBeginOverlap(Box2)
  (params (OverlappedComponent :type Primitive%20Component%20Object%20Reference) (OtherActor :type Actor%20Object%20Reference) (OtherComp :type Primitive%20Component%20Object%20Reference) (OtherBodyIndex :type Integer) (bFromSweep :type Boolean) (SweepResult :type Hit%20Result%20Structure%20%28by%20ref%29))
  (bind _cardtext (Variables|Default|GetCardText))
  (bind _text (Variables|/Script/Engine.TextRenderComponent|GetText _cardtext))
  (bind _returnvalue (Utilities|String|ToString(Text) _text))
  ;[1 1 1] az érintet jungel kártya aktiválása és az effect-jének alkalmazása arra a játékosra amelyiknek tartozik az adott munkás lap
  (if (Variables|Default|GetonBoard)
    (bind _asjungle_card (Utilities|Casting|CastToJungleCard OtherActor))
    (if (Variables|/Game/CardGameTemplate/Blueprints/Cards/Card.Card_C|GetonBoard _asjungle_card)
      (if (Utilities|Enum|Equal(Enum) _returnvalue (Utilities|String|MakeLiteralString "Blue"))
        (Default|ActivateEffect _asjungle_card)
        (elif (Utilities|Enum|Equal(Enum) _returnvalue (Utilities|String|MakeLiteralString "Red"))
          (Default|ActivateEffect _asjungle_card 1))))))

(event OnComponentBeginOverlap(Box3)
  (params (OverlappedComponent :type Primitive%20Component%20Object%20Reference) (OtherActor :type Actor%20Object%20Reference) (OtherComp :type Primitive%20Component%20Object%20Reference) (OtherBodyIndex :type Integer) (bFromSweep :type Boolean) (SweepResult :type Hit%20Result%20Structure%20%28by%20ref%29))
  (bind _cardtext (Variables|Default|GetCardText))
  (bind _text (Variables|/Script/Engine.TextRenderComponent|GetText _cardtext))
  (bind _returnvalue (Utilities|String|ToString(Text) _text))
  ;[1 1 1] az érintet jungel kártya aktiválása és az effect-jének alkalmazása arra a játékosra amelyiknek tartozik az adott munkás lap
  (if (Variables|Default|GetonBoard)
    (bind _asjungle_card (Utilities|Casting|CastToJungleCard OtherActor))
    (if (Variables|/Game/CardGameTemplate/Blueprints/Cards/Card.Card_C|GetonBoard _asjungle_card)
      (if (Utilities|Enum|Equal(Enum) _returnvalue (Utilities|String|MakeLiteralString "Blue"))
        (Default|ActivateEffect _asjungle_card)
        (elif (Utilities|Enum|Equal(Enum) _returnvalue (Utilities|String|MakeLiteralString "Red"))
          (Default|ActivateEffect _asjungle_card 1))))))

(event EventBeginPlay
  (|CallParentFunction) ; This node is disabled and will not be called.\nDrag off pins to build functionality.
)

(event Collision|EventActorBeginOverlap
  (params (OtherActor :type Actor%20Object%20Reference))
  (|CallParentFunction OtherActor) ; This node is disabled and will not be called.\nDrag off pins to build functionality.
)

(event EventTick
  (params (DeltaSeconds :type Float%20%28single-precision%29))
  (|CallParentFunction DeltaSeconds) ; This node is disabled and will not be called.\nDrag off pins to build functionality.
)

(fn ConstructionScript
  (|CallParentFunction))