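; GoldmineX1 is a card Blueprint in the card game template that grants gold to a player when its effect activates.
; ActivateEffect casts the game state to CardGameGameState, finds the pawn at the given PlayerIndex in PlayerPawns and adds the card's Gold value to that pawn's Gold.
; The other events are disabled stubs and the construction script only calls the parent.
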(event EventBeginPlay
  (|CallParentFunction) ; This node is disabled and will not be called.\nDrag off pins to build functionality.
)

(event Collision|EventActorBeginOverlap
  (params (OtherActor :type Actor%20Object%20Reference))
  (|CallParentFunction OtherActor) ; This node is disabled and will not be called.\nDrag off pins to build functionality.
)

(event EventTick
  (params (DeltaSeconds :type Float%20%28single-precision%29))
  (|CallParentFunction DeltaSeconds) ; This node is disabled and will not be called.\nDrag off pins to build functionality.
)

(event EventActivateEffect
  (params (PlayerIndex :type Integer))
  (bind _ascard_game_game_state (Utilities|Casting|CastToCardGameGameState (Game|GetGameState)))
  (Variables|/Game/CardGameTemplate/Blueprints/CardGamePawn.CardGamePawn_C|SetGold (Utilities|Array|Get(acopy) (Variables|/Game/CardGameTemplate/Blueprints/CardGameGameState.CardGameGameState_C|GetPlayerPawns _ascard_game_game_state) PlayerIndex) (+ (Variables|/Game/CardGameTemplate/Blueprints/CardGamePawn.CardGamePawn_C|GetGold (Utilities|Array|Get(acopy) (Variables|/Game/CardGameTemplate/Blueprints/CardGameGameState.CardGameGameState_C|GetPlayerPawns _ascard_game_game_state) PlayerIndex)) (Variables|Default|Getgold))))

(fn ConstructionScript
  (|CallParentFunction))