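; Temple is a card Blueprint in the card game template that awards one point to a player when its effect activates.
; ActivateEffect takes a player index and increments that player's entry in the Scores array.
; The construction script only calls its parent, and the BeginPlay, overlap and Tick events are disabled stubs.
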(event EventBeginPlay
  (|CallParentFunction) ; This node is disabled and will not be called.\nDrag off pins to build functionality.
)

(event Collision|EventActorBeginOverlap
  (params (OtherActor :type Actor%20Object%20Reference))
  (|CallParentFunction OtherActor) ; This node is disabled and will not be called.\nDrag off pins to build functionality.
)

(event EventTick
  (params (DeltaSeconds :type Float%20%28single-precision%29))
  (|CallParentFunction DeltaSeconds) ; This node is disabled and will not be called.\nDrag off pins to build functionality.
)

(event EventActivateEffect
  (params (PlayerIndex :type Integer))
  (bind _scores (Variables|Default|GetScores))
  (Utilities|Array|SetArrayElem _scores PlayerIndex (+ (Utilities|Array|Get(acopy) _scores PlayerIndex) 1)))

(fn ConstructionScript
  (|CallParentFunction))