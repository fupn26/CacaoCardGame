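; Player pawn for the card game template that owns a hand of cards and a visual Cacao counter.
; On BeginPlay, MakeHand spawns a Hand actor, stores it and attaches it to the HandAttachPoint component.
; OnCacaoChanged uses a chain of branches on the Cacao value to show that many of five Cacao components and hide the rest.
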(event EventBeginPlay
  (CallFunction|MakeHand))

(fn ConstructionScript)

(fn MakeHand
  (bind _returnvalue (Game|SpawnActorfromClass "/Game/CardGameTemplate/Blueprints/Hand.Hand_C" (Math|Transform|MakeTransform "0, 0, 0" "0, 0, 0" "1,1,1") "Undefined" 0 0))
  (bind _output_get (Variables|Hand|SetHand _returnvalue))
  (Transformation|AttachComponentToComponent _output_get (Variables|Default|GetHandAttachPoint) "None" "KeepRelative" "KeepRelative" "KeepRelative" true))

(fn OnCacaoChanged
  (bind _cacao1 (Variables|Default|GetCacao1))
  (bind _cacao2 (Variables|Default|GetCacao2))
  (bind _cacao3 (Variables|Default|GetCacao3))
  (bind _cacao4 (Variables|Default|GetCacao4))
  (bind _cacao5 (Variables|Default|GetCacao5))
  (if (== (Variables|Default|GetCacao) 0)
    (Utilities|FlowControl|Sequence
      (:then_0
        (Rendering|SetVisibility _cacao1 false false))
      (:then_1
        (Rendering|SetVisibility _cacao2 false false :!label _label))
      (:then_2
        (Rendering|SetVisibility _cacao3 false false :!label _label_2))
      (:then_3
        (Rendering|SetVisibility _cacao4 false false :!label _label_3))
      (:then_4
        (Rendering|SetVisibility _cacao5 false false :!label _label_4)))
    (elif (== (Variables|Default|GetCacao) 1)
      (Utilities|FlowControl|Sequence
        (:then_0
          (Rendering|SetVisibility _cacao1 true false :!label _label_5))
        (:then_1
          (goto _label))
        (:then_2
          (goto _label_2))
        (:then_3
          (goto _label_3))
        (:then_4
          (goto _label_4)))
      (elif (== (Variables|Default|GetCacao) 2)
        (Utilities|FlowControl|Sequence
          (:then_0
            (goto _label_5))
          (:then_1
            (Rendering|SetVisibility _cacao2 true false :!label _label_6))
          (:then_2
            (goto _label_2))
          (:then_3
            (goto _label_3))
          (:then_4
            (goto _label_4)))
        (elif (== (Variables|Default|GetCacao) 3)
          (Utilities|FlowControl|Sequence
            (:then_0
              (goto _label_5))
            (:then_1
              (goto _label_6))
            (:then_2
              (Rendering|SetVisibility _cacao3 true false :!label _label_7))
            (:then_3
              (goto _label_3))
            (:then_4
              (goto _label_4)))
          (elif (== (Variables|Default|GetCacao) 4)
            (Utilities|FlowControl|Sequence
              (:then_0
                (goto _label_5))
              (:then_1
                (goto _label_6))
              (:then_2
                (goto _label_7))
              (:then_3
                (Rendering|SetVisibility _cacao4 true false :!label _label_8))
              (:then_4
                (goto _label_4)))
            (elif (== (Variables|Default|GetCacao) 5)
              (Utilities|FlowControl|Sequence
                (:then_0
                  (goto _label_5))
                (:then_1
                  (goto _label_6))
                (:then_2
                  (goto _label_7))
                (:then_3
                  (goto _label_8))
                (:then_4
                  (Rendering|SetVisibility _cacao5 true false))))))))))