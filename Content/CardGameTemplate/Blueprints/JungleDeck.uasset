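; Jungle deck for the card game that refills the empty outer jungle card slots when clicked.
; The click handler checks both slots held on CardGameGameState and pops the deck's last card for each empty one.
; Each popped card is attached to the slot's scene component, gets an identity target transform and is stored as that slot's card.
; An unconnected leftover chain would draw from this deck into the player's hand and advance the turn.
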(event OnClicked(SelectionTrigger)
  (params (TouchedComponent :type Primitive%20Component%20Object%20Reference) (ButtonPressed :type Key%20Structure :default "None"))
  ;[1 1 1] Ha rákattintunk a jungle deckre akkor feltöltjük az üres kitett helyeket
  (bind _ascard_game_game_state (Utilities|Casting|CastToCardGameGameState (Game|GetGameState)))
  (Utilities|FlowControl|Sequence
    (:then_0
      (Utilities|IsValid (Variables|/Game/CardGameTemplate/Blueprints/BoardCardSlot.BoardCardSlot_C|GetCard (Variables|/Game/CardGameTemplate/Blueprints/CardGameGameState.CardGameGameState_C|GetOuterJungleCardSlot1 _ascard_game_game_state))
        (:Is%20Not%20Valid
          (bind _topcard (CallFunction|PopLastCard))
          (Utilities|IsValid _topcard
            (:Is%20Valid
              (Default|Attachto _topcard (Variables|/Game/CardGameTemplate/Blueprints/BoardCardSlot.BoardCardSlot_C|GetScene (Variables|/Game/CardGameTemplate/Blueprints/CardGameGameState.CardGameGameState_C|GetOuterJungleCardSlot1 _ascard_game_game_state)) false)
              (Variables|/Game/CardGameTemplate/Blueprints/Cards/Card.Card_C|SetTargetTransform _topcard (Math|Transform|MakeTransform "0, 0, 0" "0, 0, 0" "1,1,1"))
              (Variables|/Game/CardGameTemplate/Blueprints/BoardCardSlot.BoardCardSlot_C|SetCard (Variables|/Game/CardGameTemplate/Blueprints/CardGameGameState.CardGameGameState_C|GetOuterJungleCardSlot1 _ascard_game_game_state) _topcard))))))
    (:then_1
      (Utilities|IsValid (Variables|/Game/CardGameTemplate/Blueprints/BoardCardSlot.BoardCardSlot_C|GetCard (Variables|/Game/CardGameTemplate/Blueprints/CardGameGameState.CardGameGameState_C|GetOuterJungleCardSlot2 _ascard_game_game_state))
        (:Is%20Not%20Valid
          (bind _topcard_2 (CallFunction|PopLastCard))
          (Utilities|IsValid _topcard_2
            (:Is%20Valid
              (Default|Attachto _topcard_2 (Variables|/Game/CardGameTemplate/Blueprints/BoardCardSlot.BoardCardSlot_C|GetScene (Variables|/Game/CardGameTemplate/Blueprints/CardGameGameState.CardGameGameState_C|GetOuterJungleCardSlot2 _ascard_game_game_state)) false)
              (Variables|/Game/CardGameTemplate/Blueprints/Cards/Card.Card_C|SetTargetTransform _topcard_2 (Math|Transform|MakeTransform "0, 0, 0" "0, 0, 0" "1,1,1"))
              (Variables|/Game/CardGameTemplate/Blueprints/BoardCardSlot.BoardCardSlot_C|SetCard (Variables|/Game/CardGameTemplate/Blueprints/CardGameGameState.CardGameGameState_C|GetOuterJungleCardSlot2 _ascard_game_game_state) _topcard_2))))))))

(event EventBeginPlay
  (|CallParentFunction) ; This node is disabled and will not be called.\nDrag off pins to build functionality.
)

(event Collision|EventActorBeginOverlap
  (params (OtherActor :type Actor%20Object%20Reference)))

(event EventTick
  (params (DeltaSeconds :type Float%20%28single-precision%29)))

(fn ConstructionScript
  (|CallParentFunction))